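; Enemy missile projectile that homes in on the first player's pawn.
; On BeginPlay it runs the parent logic, then sets that pawn's root component as the ProjectileMovement homing target.
; Each tick it sets the mesh's world yaw from the look-at direction to the player, flipped half a turn, normalized and clamped to a forward-facing half circle.
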(event EventBeginPlay
  (|CallParentFunction)
  (Variables|/Script/Engine.ProjectileMovementComponent|SetHomingTargetComponent (Variables|Default|GetProjectileMovement) (Variables|/Script/Engine.Actor|GetRootComponent (Game|Player|GetPlayerPawn 0))))

(event EventTick
  (params (DeltaSeconds :type Float%20%28single-precision%29))
  (Transformation|SetWorldRotation (Variables|Default|GetStaticMesh1) (Math|Rotator|MakeRotator 0.0 0.0 (Math|Float|Clamp(Float) (Math|Rotator|NormalizeAxis (+ (.yaw (Math|Rotator|FindLookatRotation (Transformation|GetActorLocation) (Transformation|GetActorLocation (Game|Player|GetPlayerPawn 0)))) 1.8e+02)) -9e+01 9e+01)) false false))

(fn ConstructionScript
  (|CallParentFunction))