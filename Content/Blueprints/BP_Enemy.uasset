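; Enemy Blueprint that takes damage, shows its health on a widget health bar, and dies at zero health.
; BeginPlay caches the WBP_EnemyHealthBar from its Widget component.
; AnyDamage waits a frame, subtracts damage clamped at zero, then either updates the bar percentage or triggers death.
; Death plays a randomly pitched 2D gun sound, spawns an actor at the enemy's location, then destroys the enemy.
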(event Custom|DestroyEnemy
  ;[0.15 0.15 0.15 0.5] When enemy fire takes any damage, a sound in ranomised pitches will play
  (Utilities|FlowControl|Sequence
    (:then_0
      (Audio|PlaySound2D "/Game/Audio/Retro_Weapon_Gun_LoFi_03.Retro_Weapon_Gun_LoFi_03" 1.0 (Math|Random|RandomFloatinRange 0.5 1.5) 0.0 0 0))
    (:then_1
      (Game|SpawnActorfromClass "/Game/Particles/BP_Explosion.BP_Explosion_C" (Math|Transform|MakeTransform (Transformation|GetActorLocation) "0, 0, 0" "1.000000,1.000000,1.000000") "AlwaysSpawn" "MultiplyWithRoot" 0 0))
    (:then_2
      (Actor|DestroyActor))))

(event Custom|HitSequence
  ;[0.15 0.15 0.15 0.5] Hit sequence
  (Utilities|FlowControl|Sequence
    (:then_0
      (Default|SetHealthBarbyPercentage (Variables|Default|GetHealthBar) (/ (Variables|Default|GetHealth) (Variables|Default|GetMaxHealth))))))

(event EventBeginPlay
  ;[0.15 0.15 0.15 0.5] Set health bar once
  (bind _aswbp_enemy_health_bar (Utilities|Casting|CastToWBP_EnemyHealthBar (UserInterface|GetUserWidgetObject (Variables|Default|GetWidget))))
  (Variables|Default|SetHealthBar _aswbp_enemy_health_bar))

(event Game|Damage|EventAnyDamage
  (params (Damage :type Float%20%28single-precision%29) (DamageType :type Damage%20Type%20Object%20Reference) (InstigatedBy :type Controller%20Object%20Reference) (DamageCauser :type Actor%20Object%20Reference))
  ;[0.15 0.15 0.15 0.5] Health status
  (Utilities|FlowControl|DelayUntilNextFrame)
  (bind _output_get (Variables|Default|SetHealth (Math|Float|Max(Float) (- (Variables|Default|GetHealth) Damage) 0.0)))
  (if (== _output_get 0.0)
    (CallFunction|DestroyEnemy)
    (else
      (CallFunction|HitSequence))))

(fn ConstructionScript)