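; BP_EnemySpawner_Simple is a wave-based enemy spawner whose difficulty follows TotalScore.
; A looping timer picks an enemy class by CurrentWave, widening the random pool from Enemy A alone to A, B and C.
; Enemies spawn at a random Y between two arrow components, using the left arrow's X and rotation.
; Tick derives the wave from score thresholds and plays a sound on changes, printing a message for later waves.
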(event Custom|SpawnSpecificEnemy
  (params (EnemyToSpawn :type Actor%20Class%20Reference))
  (bind _arrowleft (Variables|Default|GetArrowLeft))
  (bind _arrowright (Variables|Default|GetArrowRight))
  (bind _returnvalue (Transformation|GetWorldLocation _arrowright))
  (bind _returnvalue_2 (Transformation|GetWorldLocation _arrowleft))
  ;[0.15 0.15 0.15 0.5] Enemy spawner location
  (Game|SpawnActorfromClass EnemyToSpawn (Math|Transform|MakeTransform (Math|Vector|MakeVector (.x _returnvalue_2) (Math|Random|RandomFloatinRange (Math|Float|Min(Float) (.y _returnvalue_2) (.y _returnvalue)) (Math|Float|Max(Float) (.y _returnvalue_2) (.y _returnvalue))) 1e+02) (Transformation|GetWorldRotation (Variables|Default|GetArrowLeft)) "1.000000,1.000000,1.000000") "AlwaysSpawn" "MultiplyWithRoot" 0 0))

(event Custom|TriggerSpawn
  ;[0.15 0.15 0.15 0.5] At begin event a a custom event will trigger and spawn enemies depending on CurrentWave what kind of enemies
  (switch int (Variables|Default|GetCurrentWave)
    (:0
      (CallFunction|SpawnSpecificEnemy "/Game/Blueprints/BP_Enemy_A.BP_Enemy_A_C" :!label _label))
    (:1
      (goto _label))
    (:2
      (CallFunction|SpawnSpecificEnemy (.OutItem (Utilities|Array|Random (Utilities|Array|MakeArray "/Game/Blueprints/BP_Enemy_A.BP_Enemy_A_C" "/Game/Blueprints/BP_Enemy_B.BP_Enemy_B_C")))))
    (:3
      (CallFunction|SpawnSpecificEnemy (.OutItem (Utilities|Array|Random (Utilities|Array|MakeArray "/Game/Blueprints/BP_Enemy_A.BP_Enemy_A_C" "/Game/Blueprints/BP_Enemy_B.BP_Enemy_B_C" "/Game/Blueprints/BP_Enemy_C.BP_Enemy_C_C")))))
    (:4
      (CallFunction|SpawnSpecificEnemy (.OutItem (Utilities|Array|Random (Utilities|Array|MakeArray "/Game/Blueprints/BP_Enemy_A.BP_Enemy_A_C" "/Game/Blueprints/BP_Enemy_B.BP_Enemy_B_C" "/Game/Blueprints/BP_Enemy_C.BP_Enemy_C_C")))))))

(event EventBeginPlay
  ;[0.15 0.15 0.15 0.5] At begin event a a custom event will trigger and spawn enemies depending on CurrentWave what kind of enemies
  (Utilities|Time|SetTimerbyEvent (delegate Custom|TriggerSpawn) 2.0 true true))

(event EventTick
  (params (DeltaSeconds :type Float%20%28single-precision%29))
  (bind _totalscore (Variables|Default|GetTotalScore))
  ;[0.15 0.15 0.15 0.5] Compare current and previous wave to play sound when new wave
  (if (!= (Variables|Default|GetCurrentWave) (Variables|Default|GetPreviousWave))
    (Audio|SpawnSound2D "/Game/Audio/Retro_Blip_07.Retro_Blip_07" 1.0 1.0 0.0 0)
    (Variables|Default|SetPreviousWave (Variables|Default|GetCurrentWave))
    (if (>= (Variables|Default|GetCurrentWave) 2)
      (Development|PrintString "New level!")))
  ;[0.15 0.15 0.15 0.5] Set new wave
  (Utilities|FlowControl|Sequence
    (:then_0
      (if (< _totalscore 10) :!label _label
        (Variables|Default|SetCurrentWave 1)))
    (:then_1
      (goto _label))
    (:then_2
      (if (and (>= _totalscore 10) (< _totalscore 30))
        (Variables|Default|SetCurrentWave 2)))
    (:then_3
      (if (and (>= _totalscore 30) (< _totalscore 50))
        (Variables|Default|SetCurrentWave 3)))
    (:then_4
      (if (>= _totalscore 50)
        (Variables|Default|SetCurrentWave 4)))))

(fn ConstructionScript)